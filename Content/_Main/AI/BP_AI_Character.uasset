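; AI soldier character for a team deathmatch that roams, hunts enemies and fights with a rifle.
; It wanders between random reachable points until Pawn Sensing spots another team's pawn, then uses AIMoveTo to close in and fire.
; A montage notify triggers muzzle effects and a damaging sphere trace.
; Death ragdolls and destroys it, with a delayed team-size update on the GameState, while Tick updates camera-facing health and team widgets.
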(event OnSeePawn(PawnSensing)
  (params (Pawn :type Pawn%20Object%20Reference))
  ;[1 1 1] Pawn Sensing
  (if (Utilities|DoesObjectImplementInterface Pawn "/Game/_Main/BP_Teamsinterface.BP_Teamsinterface_C")
    (bind _team (Class|BPTeamsinterface|GetTeam(Message) Pawn))
    (if (!= _team (Math|Conversions|ToInteger(Byte) (Variables|Default|GetTeam)))
      (bind _asbp_ai_character (Utilities|Casting|CastToBP_AI_Character Pawn)
        (:then
          (if (Variables|BP_AI_Character_C|GetIsDead _asbp_ai_character)
            (CallFunction|SearchAround)
            (else
              (CallFunction|ChaseTarget Pawn :!label _label)
              (Variables|Default|SetHasSeenTarget true))))
        (:CastFailed
          (goto _label))))))

(event Custom|Search%20Around
  ;[1 1 1] Search Around
  (if (not (Variables|Default|GetHasSeenTarget))
    (AI|AIMoveTo self (.RandomLocation (AI|Navigation|GetRandomReachablePointinRadius (Transformation|GetActorLocation) 2e+03 0 0)) 0 3e+02 false
      (:OnSuccess
        (Utilities|FlowControl|Delay 1.0)
        (CallFunction|SearchAround)))))

(event Custom|Chase%20Target
  (params (TargetActor :type Actor%20Object%20Reference))
  ;[1 1 1] Pawn Sensing
  (AI|AIMoveTo self "0, 0, 0" TargetActor 3e+02 false
    (:OnSuccess
      (CallFunction|Fire TargetActor))))

(event Custom|Fire
  (params (Target :type Actor%20Object%20Reference))
  (bind _rifle (Variables|Default|GetRifle))
  (bind _mesh (Variables|Character|GetMesh))
  (bind _returnvalue (Transformation|GetSocketTransform _rifle "b_gun_muzzleflash" "RTS_World"))
  (bind _returnvalue_2 (Transformation|GetWorldRotation _mesh))
  (if (not (Variables|Default|GetIsDead))
    (Pawn|SetControlRotation (Pawn|GetController) (Math|Rotator|FindLookatRotation (Transformation|GetActorLocation) (Transformation|GetActorLocation Target)))
    (Animation|Montage|PlayMontage (Variables|Character|GetMesh) "/Game/_Main/Animations/Animation_Assets/IronSight_Shoot.IronSight_Shoot"
      (:OnNotifyBegin
        (Effects|SpawnEmitterAttached "/Game/MilitaryWeapSilver/FX/P_AssaultRifle_MuzzleFlash.P_AssaultRifle_MuzzleFlash" (Variables|Default|GetRifle) "b_gun_muzzleflash" (.location _returnvalue) _returnvalue_2 "1.000000,1.000000,1.000000" "KeepWorldPosition" true "AutoRelease")
        (Audio|PlaySoundatLocation "/Game/_Main/Audio/MS_Rifle.MS_Rifle" (Transformation|GetActorLocation) "0, 0, 0" 0.6 1.0 0.0 0 0 0 0)
        (bind (_outhit _returnvalue_3) (Collision|SphereTraceByChannel (.location _returnvalue) (+ (.location _returnvalue) (* (Math|Vector|GetRightVector _returnvalue_2) 3e+03)) 15.0 "TraceTypeQuery1" false 0 "None" false))
        (if _returnvalue_3
          (Game|Damage|ApplyDamage (.HitActor (Collision|BreakHitResult _outhit)) 1e+01 0 0)
          (Effects|SpawnEmitteratLocation "/Game/Realistic_Starter_VFX_Pack_Vol2/Particles/Blood/P_Blood_Splat_Cone.P_Blood_Splat_Cone" (.ImpactPoint (Collision|BreakHitResult _outhit))))))))

(event EventBeginPlay
  ;[1 1 1] Begin Play
  (Utilities|FlowControl|Delay 1e+01)
  (CallFunction|SearchAround)
  (Utilities|FlowControl|Sequence
    (:then_0
      (if (== (Variables|Default|GetTeam) 1)
        (bind _asai_teams (Utilities|Casting|CastToAI_Teams (UserInterface|GetWidget (Variables|Default|GetTeamWidget))))
        (Rendering|Components|TextRender|SetText (Variables|/Game/_Main/UI/AI_UserInterface/AI_Teams.AI_Teams_C|GetTeam_text _asai_teams) "Team B")))
    (:then_1
      (Utilities|FlowControl|Delay 0.3 :!label _label)
      (if (Variables|Default|GetHasSeenTarget)
        (CallFunction|SearchAround)
        (Variables|Default|SetHasSeenTarget false)
        (goto _label)))))

(event Game|Damage|EventAnyDamage
  (params (Damage :type Float%20%28single-precision%29) (DamageType :type Damage%20Type%20Object%20Reference) (InstigatedBy :type Controller%20Object%20Reference) (DamageCauser :type Actor%20Object%20Reference))
  ;[1 1 1] Apply Damage
  (Variables|Default|SetHealth (- (Variables|Default|GetHealth) Damage))
  (if (<= (Variables|Default|GetHealth) 0.0)
    (Utilities|FlowControl|DoOnce false
      (:Completed
        (Physics|SetSimulatePhysics (Variables|Character|GetMesh) true)
        (Variables|Default|SetIsDead true)
        (Rendering|SetVisibility (Variables|Default|GetHealthBar) false false)
        (Utilities|FlowControl|Delay 2.0)
        (Actor|DestroyActor)
        (Utilities|FlowControl|Delay 2.0)
        (bind _asgs_team_deathmatch (Utilities|Casting|CastToGS_TeamDeathmatch (Game|GetGameState)))
        (Default|DecreaseTeamSize _asgs_team_deathmatch (== (Variables|Default|GetTeam) 0))))))

(event EventTick
  (params (DeltaSeconds :type Float%20%28single-precision%29))
  ;[1 1 1] HealthBar Update
  (bind _asai_health_bar (Utilities|Casting|CastToAI_HealthBar (UserInterface|GetWidget (Variables|Default|GetHealthBar))))
  (Progress|SetPercent (Variables|/Game/_Main/UI/AI_UserInterface/AI_HealthBar.AI_HealthBar_C|GetHealthbar _asai_health_bar) (/ (Variables|Default|GetHealth) 1e+02))
  (Transformation|SetWorldRotation (Variables|Default|GetHealthBar) (Math|Rotator|FindLookatRotation (Transformation|GetActorLocation) (Transformation|GetActorLocation (Game|GetPlayerCameraManager 0))) false false))

(event EventSetTeam
  (params (Team :type E_Teams%20Enum :default "NewEnumerator0"))
  ;[1 1 1] Set Team
  (Variables|Default|SetTeam Team))

(fn ConstructionScript)

(fn GetTeam
  (return (Variables|Default|GetTeam)))